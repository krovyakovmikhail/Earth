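; BP_SunManager drives the sun's movement by rotating a referenced DirectionalLight and BPSun actor together.
; On BeginPlay, once both references are valid, it starts a looping timer in place of Tick.
; Each timer pulse adds SunSpeed as a world yaw delta to both actors, so rotation advances in fixed steps without delta-time scaling.
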(event `self.ReceiveBeginPlay`
  (`self.DirectionalLight`
    (:`then`
      (`self.BP_Sun`
        (:`then`
          (`KismetSystemLibrary.K2_SetTimerDelegate` (delegate `Cycle`) 0.1 true))
        (:`else`)))
    (:`else`)))

(event `Cycle`
  (`self.K2_AddActorWorldRotation` (`self.DirectionalLight`) (`KismetMathLibrary.MakeRotator` 0.0 0.0 (`self.SunSpeed`)) false false)
  (`self.K2_AddActorWorldRotation` (`self.BP_Sun`) (`KismetMathLibrary.MakeRotator` 0.0 0.0 (`self.SunSpeed`)) false false))

(fn `UserConstructionScript`)