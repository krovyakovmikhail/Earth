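; Player controller that drives an orbit-and-zoom camera on the spring arm of BP_MainPAwn, with the mouse cursor shown.
; While the right mouse button is held, look axes rotate the arm in fixed steps of DeltaRotationSpeed, with pitch limited short of vertical.
; The mouse wheel changes arm length within limits and adjusts rotation speed to match, slower when closer, printing the new speed for debugging.
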(event `self.ReceiveTick`
  (params (DeltaSeconds :type "Float (single-precision)")))

(event `self.ReceiveBeginPlay`
  (bind _asbp_main_pawn (cast `/Game/Dev/Main/BP_MainPAwn` (`self.K2_GetPawn`)))
  (set `self.As BP Main PAwn` _asbp_main_pawn)
  (set `self.bShowMouseCursor` true))

(event `InputAxis|LooAround`
  (params (AxisValue :type "Float (single-precision)"))
  (bind _delta_rotation_speed_ (`self.Delta Rotation Speed `))
  (if (> (`KismetMathLibrary.Abs` AxisValue) 0.03)
    (if (`self.RMB_Pressed`)
      (bind _as_bp_main_pawn (`self.As BP Main PAwn`)
        (:`then`
          (if (> AxisValue 0.0)
            (bind _springarm (`/Game/Dev/Main/BP_MainPAwn.SpringArm` _as_bp_main_pawn))
            (`SceneComponent.K2_AddRelativeRotation` _springarm (`KismetMathLibrary.MakeRotator` 0.0 0.0 (* _delta_rotation_speed_ 1.0)) false false)
            (elif (< AxisValue 0.0)
              (`SceneComponent.K2_AddRelativeRotation` _springarm (`KismetMathLibrary.MakeRotator` 0.0 0.0 (* _delta_rotation_speed_ -1.0)) false false))))
        (:`else`)))))

(event `InputAxis|LookUPDown`
  (params (AxisValue :type "Float (single-precision)"))
  (bind _delta_rotation_speed_ (`self.Delta Rotation Speed `))
  (if (`self.RMB_Pressed`)
    (bind _as_bp_main_pawn (`self.As BP Main PAwn`)
      (:`then`
        (bind _springarm (`/Game/Dev/Main/BP_MainPAwn.SpringArm` _as_bp_main_pawn))
        (bind (_returnvalue_roll _returnvalue_pitch) (`KismetMathLibrary.BreakRotator` (`SceneComponent.K2_GetComponentRotation` _springarm)))
        (if (and (< AxisValue 0.0) (> _returnvalue_pitch -88.0))
          (`SceneComponent.K2_AddRelativeRotation` _springarm (`KismetMathLibrary.MakeRotator` 0.0 (* _delta_rotation_speed_ -1.0)) false false)
          (elif (and (> AxisValue 0.0) (< _returnvalue_pitch 88.0))
            (`SceneComponent.K2_AddRelativeRotation` _springarm (`KismetMathLibrary.MakeRotator` 0.0 (* _delta_rotation_speed_ 1.0)) false false))))
      (:`else`))))

(event `InputAction|MouseButtonRight`
  (params (Key :type "Key Structure"))
  (:`Pressed`
    (set `self.RMB_Pressed` true))
  (:`Released`
    (set `self.RMB_Pressed` false)))

(event `InputAxis|MouseWheelAxis`
  (params (AxisValue :type "Float (single-precision)"))
  (bind _delta_rotation_speed_ (`self.Delta Rotation Speed `))
  (bind _delta_rotation_speed__2 (`self.Delta Rotation Speed `))
  (bind _returnvalue (- _delta_rotation_speed__2 0.05))
  (if (> AxisValue 0.0)
    (bind _as_bp_main_pawn (`self.As BP Main PAwn`)
      (:`then`
        (bind _springarm (`/Game/Dev/Main/BP_MainPAwn.SpringArm` _as_bp_main_pawn))
        (bind _returnvalue_2 (+ (`SpringArmComponent.TargetArmLength` _springarm) (* AxisValue -5000.0)))
        (if (> _returnvalue_2 340000.0)
          (set `SpringArmComponent.TargetArmLength` _returnvalue_2 _springarm)
          (if (>= _returnvalue 0.05)
            (bind _output_get (set `self.Delta Rotation Speed ` (`KismetMathLibrary.Lerp` _delta_rotation_speed__2 _returnvalue 0.5)))
            (`KismetSystemLibrary.PrintString` (`KismetStringLibrary.Conv_DoubleToString` _output_get)))))
      (:`else`))
    (elif (< AxisValue 0.0)
      (if (< _returnvalue_2 800000.0)
        (set `SpringArmComponent.TargetArmLength` _returnvalue_2 _springarm)
        (bind _output_get_2 (set `self.Delta Rotation Speed ` (`KismetMathLibrary.Lerp` _delta_rotation_speed_ (+ _delta_rotation_speed_ 0.05) 0.5)))
        (`KismetSystemLibrary.PrintString` (`KismetStringLibrary.Conv_DoubleToString` _output_get_2))))))

(fn `UserConstructionScript`)